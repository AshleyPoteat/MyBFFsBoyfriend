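; BP_Disposal is a disposal point that takes in body parts through an overlap box.
; Until full, it destroys any overlapping non-player actor without a type check and increments a body part count.
; At six it marks itself full and calls HidTheBody on the Wid_PlayerTimer widget.
; A Tick player check leads only to an empty DoOnce, and a pause-and-confirm widget chain is left disconnected.
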(event `self.Box.OnComponentBeginOverlap`
  (params (OverlappedComponent :type "PrimitiveComponent Object Reference") (OtherActor :type "Actor Object Reference") (OtherComp :type "PrimitiveComponent Object Reference") (OtherBodyIndex :type Integer) (bFromSweep :type Boolean) (SweepResult :type "HitResult Structure (by ref)"))
  (if (`self.isFull?`)
    _
    (elif (not (== OtherActor (`GameplayStatics.GetPlayerCharacter` 0)))
      (`self.K2_DestroyActor` OtherActor)
      (bind _result (`/Engine/EditorBlueprintResources/StandardMacros.IncrementFloat` (`self.bodyParts`))
        (:`  `
          (set `self.bodyParts` _result)
          (if (== (`self.bodyParts`) 6.0)
            (set `self.isFull?` true)
            (bind _foundwidgets (`WidgetBlueprintLibrary.GetAllWidgetsOfClass` "/Game/MMetcalf/Checklist/Wid_PlayerTimer.Wid_PlayerTimer_C"))
            (`/Game/MMetcalf/Checklist/Wid_PlayerTimer.HidTheBody` _foundwidgets)))))))

(event `self.ReceiveTick`
  (params (DeltaSeconds :type "Float (single-precision)"))
  (if (== (stale `self.Box.OnComponentBeginOverlap` OtherActor) (`GameplayStatics.GetPlayerCharacter` 0))
    (`/Engine/EditorBlueprintResources/StandardMacros.DoOnce` false)))

(fn `UserConstructionScript`)