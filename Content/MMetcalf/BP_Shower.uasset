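; Interactable shower that the player uses once, through a prompt widget and interact input enabled while inside its Box trigger.
; Interact plays the shower sound on every press, but a DoOnce limits the rest: set DidShower, hide the prompt, freeze movement briefly, then notify Wid_PlayerTimer.
; DidShower stops both overlap handlers, so input stays enabled after showering.
; LastThing! clears DidShower without resetting the DoOnce.
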(event `InputAction|IA_Interact`
  (params (Key :type "Key Structure"))
  (bind _charactermovement (`Character.CharacterMovement` (`GameplayStatics.GetPlayerCharacter` 0)))
  (:`Pressed`
    (`GameplayStatics.PlaySound2D` "/Game/APoteat/Sounds/showering_Cue.showering_Cue" 1.0 1.0 0.0 null null)
    (`/Engine/EditorBlueprintResources/StandardMacros.DoOnce` false
      (:`Completed`
        (set `self.DidShower?` true)
        (`SceneComponent.SetVisibility` (`self.Widget`) false false)
        (`CharacterMovementComponent.DisableMovement` _charactermovement)
        (`KismetSystemLibrary.Delay` 5.0)
        (`CharacterMovementComponent.SetMovementMode` _charactermovement "MOVE_Walking" 0)
        (bind _foundwidgets (`WidgetBlueprintLibrary.GetAllWidgetsOfClass` "/Game/MMetcalf/Checklist/Wid_PlayerTimer.Wid_PlayerTimer_C"))
        (`/Game/MMetcalf/Checklist/Wid_PlayerTimer.DidShower` _foundwidgets)))))

(event `self.ReceiveBeginPlay`
  (`SceneComponent.SetVisibility` (`self.Widget`) false false))

(event `self.Box.OnComponentBeginOverlap`
  (params (OverlappedComponent :type "PrimitiveComponent Object Reference") (OtherActor :type "Actor Object Reference") (OtherComp :type "PrimitiveComponent Object Reference") (OtherBodyIndex :type Integer) (bFromSweep :type Boolean) (SweepResult :type "HitResult Structure (by ref)"))
  (if (== OtherActor (`GameplayStatics.GetPlayerCharacter` 0))
    (if (not (`self.DidShower?`))
      (`self.EnableInput` (`GameplayStatics.GetPlayerController` 0))
      (`SceneComponent.SetVisibility` (`self.Widget`) true false))))

(event `self.Box.OnComponentEndOverlap`
  (params (OverlappedComponent :type "PrimitiveComponent Object Reference") (OtherActor :type "Actor Object Reference") (OtherComp :type "PrimitiveComponent Object Reference") (OtherBodyIndex :type Integer))
  (if (== OtherActor (`GameplayStatics.GetPlayerCharacter` 0))
    (if (not (`self.DidShower?`))
      (`self.DisableInput` (`GameplayStatics.GetPlayerController` 0))
      (`SceneComponent.SetVisibility` (`self.Widget`) false false))))

(event `LastThing!`
  (set `self.DidShower?` false))

(fn `UserConstructionScript`)